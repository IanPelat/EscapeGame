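; Fireball launcher trap that automatically fires BP_FireballProjectile from its projectile start position at a repeating interval.
; Tick counts down the current cooldown through the projectile spawn component, then has that component fire and resets the cooldown to the configured value.
; Firing is purely timer-driven, with no trigger, targeting or overlap logic in the graph.
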(event `self.ReceiveTick`
  (params (DeltaSeconds :type "Float (single-precision)"))
  ;[1 1 1] Fire Projectile CD
  (if (> (`self.FireProjectionCurrentCD`) 0.0)
    (bind _newcd (`/Game/EscapeGame/Core/Abilities/BP_Abilities.CDTick` (`self.BP_ProjectileSpawnComponent`) (`self.FireProjectionCurrentCD`) DeltaSeconds))
    (set `self.FireProjectionCurrentCD` _newcd)
    (else
      ;[1 1 1] Fire Projectile
      (`/Game/EscapeGame/Core/Projectile/BP_ProjectileSpawnComponent.FireProjectile` (`self.BP_ProjectileSpawnComponent`) "/Game/EscapeGame/Projectiles/Fireball/BP_FireballProjectile.BP_FireballProjectile_C" (`self.ProjectileStartPosition`))
      (set `self.FireProjectionCurrentCD` (`self.FireProjectileCD`)))))

(fn `UserConstructionScript`)